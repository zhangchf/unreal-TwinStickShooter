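; Enemy character Blueprint that repeatedly damages the hero on overlap and dies when its own health runs out.
; Overlapping a HeroCharacter starts a looping timer at the attack rate that applies damage, cleared when the hero leaves.
; AffectHealth updates and prints health; on death it ignores key collision channels, detaches the controller and destroys itself after a delay.
; The construction script tints the mesh through the BodyColor material parameter.
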(event `self.ReceiveActorBeginOverlap`
  (params (OtherActor :type "Actor Object Reference"))
  ;[1 1 1] Attack
  (bind _ashero_character (cast `/Game/Blueprints/HeroCharacter` OtherActor))
  (set `self.Hero` _ashero_character)
  (bind _returnvalue (`KismetSystemLibrary.K2_SetTimer` null "InflictDamage" (/ 1.0 (`self.AttacksPerSecond`)) true))
  (set `self.AttackTimer` _returnvalue))

(event `InflictDamage`
  ;[1 1 1] Attack
  (`/Game/Blueprints/IDamageable.AffectHealth` (`self.Hero`) (`self.Damage`)))

(event `self.ReceiveActorEndOverlap`
  (params (OtherActor :type "Actor Object Reference"))
  ;[1 1 1] Cease Attack
  (if (== OtherActor (`self.Hero`))
    (`KismetSystemLibrary.K2_ClearAndInvalidateTimerHandle` (`self.AttackTimer`))))

(event `/Game/Blueprints/IDamageable.AffectHealth`
  (params (Delta :type "Float (single-precision)"))
  (bind _capsulecomponent (`self.CapsuleComponent`))
  ;[1 1 1] TakeDamage and Die
  (`self.CalculateHealth` Delta)
  (`KismetSystemLibrary.PrintString` (`KismetStringLibrary.Conv_DoubleToString` (`self.Health`)))
  (if (`self.isDead`)
    ;;[1 1 1] Disable Collision
    (`PrimitiveComponent.SetCollisionResponseToChannel` _capsulecomponent "ECC_WorldDynamic" "ECR_Ignore")
    (`PrimitiveComponent.SetCollisionResponseToChannel` _capsulecomponent "ECC_Pawn" "ECR_Ignore")
    ;;[1 1 1] Disable AI Move
    (`self.DetachFromControllerPendingDestroy`)
    (`KismetSystemLibrary.Delay` 3.0)
    (`self.K2_DestroyActor`)))

(fn `UserConstructionScript`
  (locals (DynaMat :type "MaterialInterface Object Reference"))
  (set `local.DynaMat` (`PrimitiveComponent.GetMaterialFromCollisionFaceIndex` (`self.Mesh`) 0))
  (`MeshComponent.SetVectorParameterValueOnMaterials` (`self.Mesh`) "BodyColor" (`KismetMathLibrary.Conv_LinearColorToVector` (`self.BodyColor`))))