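; Weapon Blueprint that fires projectiles automatically at a set rate while its trigger is held.
; PullTrigger starts a looping timer at an interval derived from RoundsPerSecond, with a DoOnce blocking repeat starts and the first shot coming one interval later.
; Each timer tick calls Fire, which spawns the Projectile class at the ProjectileSpawnPoint transform.
; ReleaseTrigger clears the timer and resets the DoOnce.
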(event `PullTrigger`
  (`/Engine/EditorBlueprintResources/StandardMacros.DoOnce` false :!label _label
    (:`Completed`
      (bind _returnvalue (`KismetSystemLibrary.K2_SetTimerDelegate` (delegate `Fire`) (/ 1.0 (`self.RoundsPerSecond`)) true))
      (set `self.FireTimer` _returnvalue))))

(event `ReleaseTrigger`
  (`KismetSystemLibrary.K2_ClearAndInvalidateTimerHandle` (`self.FireTimer`))
  (goto _label :!via `Reset`))

(event `Fire`
  (`|SpawnActorFromClass` "/Game/Blueprints/Projectile.Projectile_C" (`SceneComponent.K2_GetComponentToWorld` (`self.ProjectileSpawnPoint`)) "Undefined" "OverrideRootScale"))

(fn `UserConstructionScript`)